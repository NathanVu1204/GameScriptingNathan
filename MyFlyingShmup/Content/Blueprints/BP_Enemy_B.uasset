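; BP_Enemy_B is an enemy Blueprint that fires BP_EnemyBullet actors continuously from its BulletSpawnPoint.
; BeginPlay starts a looping timer that calls ShootBullet every second.
; ShootBullet spawns three bullets separated by Delay nodes, a sequence longer than the timer interval, so successive volleys overlap.
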(event Custom|ShootBullet
  (Game|SpawnActorfromClass "/Game/Blueprints/BP_EnemyBullet.BP_EnemyBullet_C" (Transformation|GetWorldTransform (Variables|Default|GetBulletSpawnPoint)) "Undefined" "MultiplyWithRoot" 0 0)
  (Utilities|FlowControl|Delay 0.75)
  (Game|SpawnActorfromClass "/Game/Blueprints/BP_EnemyBullet.BP_EnemyBullet_C" (Transformation|GetWorldTransform (Variables|Default|GetBulletSpawnPoint)) "Undefined" "MultiplyWithRoot" 0 0)
  (Utilities|FlowControl|Delay 0.75)
  (Game|SpawnActorfromClass "/Game/Blueprints/BP_EnemyBullet.BP_EnemyBullet_C" (Transformation|GetWorldTransform (Variables|Default|GetBulletSpawnPoint)) "Undefined" "MultiplyWithRoot" 0 0))

(event EventBeginPlay
  (Utilities|Time|SetTimerbyEvent (delegate Custom|ShootBullet) 1.0 true true))

(fn ConstructionScript)