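; BP_EnemyTurret is an enemy turret actor that turns to face the player and fires bullets at regular intervals.
; Every tick it yaws TurretBase toward player pawn 0 using a look-at rotation, keeping pitch and roll at zero.
; A looping timer started on BeginPlay spawns a BP_EnemyBullet at the Scene component's world transform, regardless of collisions, with no range or line-of-sight check.
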(event Custom|ShootBullet
  (Game|SpawnActorfromClass "/Game/Blueprints/BP_EnemyBullet.BP_EnemyBullet_C" (Transformation|GetWorldTransform (Variables|Default|GetScene)) "AlwaysSpawn" "MultiplyWithRoot" 0 0))

(event EventBeginPlay
  (|CallParentFunction)
  (Utilities|Time|SetTimerbyEvent (delegate Custom|ShootBullet) 2.75 true true))

(event Collision|EventActorBeginOverlap
  (params (OtherActor :type Actor%20Object%20Reference))
  (|CallParentFunction OtherActor) ; This node is disabled and will not be called.\nDrag off pins to build functionality.
)

(event EventTick
  (params (DeltaSeconds :type Float%20%28single-precision%29))
  (Transformation|SetWorldRotation (Variables|Default|GetTurretBase) (Math|Rotator|MakeRotator 0.0 0.0 (.yaw (Math|Rotator|FindLookatRotation (Transformation|GetActorLocation) (Transformation|GetActorLocation (Game|Player|GetPlayerPawn 0))))) false false))

(fn ConstructionScript
  (|CallParentFunction))