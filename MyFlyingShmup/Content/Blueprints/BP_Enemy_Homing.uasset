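; BP_Enemy_Homing is an enemy that continuously chases the first player's pawn.
; Every Tick it feeds the unit direction toward that pawn into its FloatingPawnMovement as movement input.
; It also turns to face the target using only the yaw of a look-at rotation, while the movement direction keeps its vertical component.
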(event EventBeginPlay
  (|CallParentFunction) ; This node is disabled and will not be called.\nDrag off pins to build functionality.
)

(event Collision|EventActorBeginOverlap
  (params (OtherActor :type Actor%20Object%20Reference))
  (|CallParentFunction OtherActor) ; This node is disabled and will not be called.\nDrag off pins to build functionality.
)

(event EventTick
  (params (DeltaSeconds :type Float%20%28single-precision%29))
  (bind _returnvalue (Game|Player|GetPlayerPawn 0))
  (bind _returnvalue_2 (Transformation|GetActorLocation))
  (bind _returnvalue_3 (Transformation|GetActorLocation _returnvalue))
  (Class|PawnMovementComponent|AddInputVector (Variables|Default|GetFloatingPawnMovement) (Math|Vector|GetUnitDirection(Vector) _returnvalue_2 _returnvalue_3) false)
  (Transformation|SetActorRotation (Math|Rotator|MakeRotator 0.0 0.0 (.yaw (Math|Rotator|FindLookatRotation _returnvalue_2 _returnvalue_3)))))

(fn ConstructionScript
  (|CallParentFunction))