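; BP_EnemyBoss1 is a boss enemy that flies or slides into the play area, then moves sideways.
; On BeginPlay it runs the parent logic, then a timeline offsets it along negative X from its spawn location.
; When that finishes, it stores its new location and a slowed timeline drives movement along Y.
; Both moves set the actor location with sweep, relative to the stored start point.
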(event Custom|MoveSideToSide
  (Variables|Default|SetInitialLocation (Transformation|GetActorLocation))
  (Components|Timeline|SetPlayRate (Variables|Default|GetTL_MoveSideToSide) 0.05)
  (bind _newtrack_0 (Timeline|TL_MoveSideToSide PlayFromStart)
    (:Update
      (Transformation|SetActorLocation (+ (Variables|Default|GetInitialLocation) (Math|Vector|MakeVector 0.0 (* _newtrack_0 3e+03) 0.0)) true false))))

(event Custom|EnterPlayArea
  (Variables|Default|SetInitialLocation (Transformation|GetActorLocation))
  (bind _newtrack_0 (Timeline|TL_EnterPlayArea PlayFromStart)
    (:Update
      (Transformation|SetActorLocation (+ (Variables|Default|GetInitialLocation) (Math|Vector|MakeVector (* _newtrack_0 -1.8e+03) 0.0 0.0)) true false))
    (:Finished
      (CallFunction|MoveSidetoSide))))

(event EventBeginPlay
  (|CallParentFunction)
  (CallFunction|EnterPlayArea))

(fn ConstructionScript
  (|CallParentFunction))